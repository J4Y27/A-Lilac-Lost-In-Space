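; BP_Enemy is a patrolling enemy character that walks forward every tick and deals contact damage to actors not tagged IGNORE.
; Wall and ledge detector overlaps call TurnChar to reverse its facing, printing the other actor's name for debugging.
; Overlapping a LedgeWall-tagged actor also flips it and issues an AI move along X.
; Damage lowers its clamped health; at zero it spawns a Niagara effect and destroys itself.
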(event OnComponentBeginOverlap(WalDetector)
  (params (OverlappedComponent :type Primitive%20Component%20Object%20Reference) (OtherActor :type Actor%20Object%20Reference) (OtherComp :type Primitive%20Component%20Object%20Reference) (OtherBodyIndex :type Integer) (bFromSweep :type Boolean) (SweepResult :type Hit%20Result%20Structure%20%28by%20ref%29))
  (Development|PrintString (Utilities|GetDisplayName OtherActor))
  (CallFunction|TurnChar))

(event OnComponentHit(CapsuleComponent)
  (params (HitComponent :type Primitive%20Component%20Object%20Reference) (OtherActor :type Actor%20Object%20Reference) (OtherComp :type Primitive%20Component%20Object%20Reference) (NormalImpulse :type Vector :default "0, 0, 0") (Hit :type Hit%20Result%20Structure%20%28by%20ref%29))
  (if (not (Actor|ActorHasTag OtherActor "IGNORE"))
    (Game|Damage|ApplyDamage OtherActor 1.0 0 0)))

(event OnComponentEndOverlap(LedgeDetector)
  (params (OverlappedComponent :type Primitive%20Component%20Object%20Reference) (OtherActor :type Actor%20Object%20Reference) (OtherComp :type Primitive%20Component%20Object%20Reference) (OtherBodyIndex :type Integer))
  (Development|PrintString (Utilities|GetDisplayName OtherActor))
  (CallFunction|TurnChar))

(event EventBeginPlay)

(event Collision|EventActorBeginOverlap
  (params (OtherActor :type Actor%20Object%20Reference))
  (if (Actor|ActorHasTag OtherActor "LedgeWall")
    (Transformation|SetActorRotation (Math|Rotator|CombineRotators (Transformation|GetActorRotation) "0.000000,-180.000000,0.000000"))
    (AI|Navigation|MovetoLocation (AI|GetAIController 0) (+ (Transformation|GetActorLocation) (* (Transformation|GetActorForwardVector) "500.000000,0.000000,0.000000")) -1.0 true true false true 0)))

(event EventTick
  (params (DeltaSeconds :type Float%20%28single-precision%29))
  (Pawn|Input|AddMovementInput (Transformation|GetActorForwardVector) 1.0 false))

(event Game|Damage|EventAnyDamage
  (params (Damage :type Float%20%28single-precision%29) (DamageType :type Damage%20Type%20Object%20Reference) (InstigatedBy :type Controller%20Object%20Reference) (DamageCauser :type Actor%20Object%20Reference))
  (bind _output_get (Variables|Default|SetCurrentHEalth (Math|Float|Truncate (Math|Float|Clamp(Float) (- (Variables|Default|GetCurrentHEalth) Damage) 0.0 (Math|Conversions|ToFloat(Integer) (Variables|Default|GetMaxHealth))))))
  (if (<= _output_get 0)
    (Niagara|SpawnSystematLocation "/Game/Jamar_B/Effects/Niagra/NS_FX.NS_FX" (Transformation|GetActorLocation))
    (Actor|DestroyActor)))

(fn ConstructionScript)

(fn TurnChar
  (Transformation|SetActorRotation (Math|Rotator|CombineRotators (Transformation|GetActorRotation) "0.000000,180.000000,0.000000")))