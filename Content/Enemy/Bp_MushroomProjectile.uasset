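; Enemy mushroom projectile that flies along its shoot direction and damages Lyla on contact.
; Movement is manual: CharacterMovement is deactivated and Tick offsets the actor after a short look-ahead line trace against world objects.
; A hit reverses the direction and flips the sprite to match, destroying the projectile once it exceeds its bounce limit.
; Capsule overlap with Lyla applies damage and destroys it.
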(event OnComponentBeginOverlap(CapsuleComponent)
  (params (OverlappedComponent :type Primitive%20Component%20Object%20Reference) (OtherActor :type Actor%20Object%20Reference) (OtherComp :type Primitive%20Component%20Object%20Reference) (OtherBodyIndex :type Integer) (bFromSweep :type Boolean) (SweepResult :type Hit%20Result%20Structure%20%28by%20ref%29))
  (Utilities|Casting|CastToBp_Lyla OtherActor)
  (Game|Damage|ApplyDamage OtherActor 1.0 0 self)
  (Actor|DestroyActor))

(event EventBeginPlay
  (Components|Activation|Deactivate (Variables|Character|GetCharacterMovement))
  (if (< (.X (Math|Vector|BreakVector (Variables|Default|GetShootDirection))) 0.0)
    (Transformation|SetRelativeRotation (Variables|Default|GetSprite) "0.000000,180.000000,0.000000" false false)
    (else
      (Transformation|SetRelativeRotation (Variables|Default|GetSprite) "0, 0, 0" false false))))

(event Collision|EventActorBeginOverlap
  (params (OtherActor :type Actor%20Object%20Reference)))

(event EventTick
  (params (DeltaSeconds :type Float%20%28single-precision%29))
  (bind _speed (Variables|Default|GetSpeed))
  (bind _returnvalue (Class|KismetSystemLibrary|LineTraceMultiforObjects (Transformation|GetActorLocation) (+ (Transformation|GetActorLocation) (* (Variables|Default|GetShootDirection) (+ (* _speed DeltaSeconds) 2e+01))) (Utilities|Array|MakeArray "ObjectTypeQuery1" "ObjectTypeQuery2") false (Utilities|Array|MakeArray self) "None" true))
  (if _returnvalue
    (Variables|Default|SetBounceCount (+ (Variables|Default|GetBounceCount) 1))
    (if (> (Variables|Default|GetBounceCount) (Variables|Default|GetMaxBounces))
      (Actor|DestroyActor)
      (else
        (Variables|Default|SetShootDirection (* (Variables|Default|GetShootDirection) -1.0))
        (if (< (.X (Math|Vector|BreakVector (Variables|Default|GetShootDirection))) 0.0)
          (Transformation|SetRelativeRotation (Variables|Default|GetSprite) "0.000000,180.000000,0.000000" false false)
          (else
            (Transformation|SetRelativeRotation (Variables|Default|GetSprite) "0, 0, 0" false false)))
        (Transformation|AddActorWorldOffset (* (Variables|Default|GetShootDirection) _speed DeltaSeconds) :!label _label)))
    (else
      (goto _label))))

(fn ConstructionScript)