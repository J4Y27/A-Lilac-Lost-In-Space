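; MushroomEnemy is a stationary-style 2D flipbook enemy that periodically shoots at the player and can be killed by damage.
; A looping timer fires when the player is within range, playing an attack flipbook, spawning a projectile aimed left or right along X toward the player, then returning to the breathing loop.
; AnyDamage reduces clamped health and, at zero, spawns a Niagara effect and destroys the actor.
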(event Custom|Fire
  (bind _sprite (Variables|Default|GetSprite))
  (bind _sprite_2 (Variables|Default|GetSprite))
  (if (<= (Transformation|GetDistanceTo (Game|Player|GetPlayerPawn 0)) (Variables|Default|GetShootRange))
    (Sprite|SetFlipbook _sprite "/Game/Jamar_B/Enemies/Mushroom/Mushroom_Attack/Mushroom_Attack.Mushroom_Attack")
    (Components|Timeline|SetLooping _sprite false)
    (Components|Timeline|PlayfromStart _sprite)
    (Utilities|FlowControl|Delay 0.3)
    (Game|SpawnActorfromClass "/Game/Enemy/Bp_MushroomProjectile.Bp_MushroomProjectile_C" (Math|Transform|MakeTransform (Transformation|GetWorldLocation (Variables|Default|GetBulletSpawn))) "AlwaysSpawn" "MultiplyWithRoot" 0 (Math|Vector|MakeVector (Math|Float|Sign(Float) (- (.X (Math|Vector|BreakVector (Transformation|GetActorLocation (Game|Player|GetPlayerPawn 0)))) (.X (Math|Vector|BreakVector (Transformation|GetActorLocation))))) 0.0 0.0) 0)
    (Utilities|FlowControl|Delay 0.5)
    (Sprite|SetFlipbook _sprite_2 "/Game/Jamar_B/Enemies/Mushroom/Mushroom_Breathing/Mushroom_Breathing.Mushroom_Breathing")
    (Components|Timeline|SetLooping _sprite_2 true)
    (Audio|Components|Audio|Play _sprite_2)))

(event EventBeginPlay
  (Variables|Default|SetCurrent%20HEalth (Variables|Default|GetMax%20Health))
  (Utilities|Time|SetTimerbyEvent (delegate Custom|Fire) (Variables|Default|GetFireInterval) true))

(event Collision|EventActorBeginOverlap
  (params (OtherActor :type Actor%20Object%20Reference)))

(event EventTick
  (params (DeltaSeconds :type Float%20%28single-precision%29)))

(event Game|Damage|EventAnyDamage
  (params (Damage :type Float%20%28single-precision%29) (DamageType :type Damage%20Type%20Object%20Reference) (InstigatedBy :type Controller%20Object%20Reference) (DamageCauser :type Actor%20Object%20Reference))
  (bind _output_get (Variables|Default|SetCurrent%20HEalth (Math|Float|Truncate (Math|Float|Clamp(Float) (- (Variables|Default|GetCurrent%20HEalth) Damage) 0.0 (Math|Conversions|ToFloat(Integer) (Variables|Default|GetMax%20Health))))))
  (if (<= _output_get 0)
    (Niagara|SpawnSystematLocation "/Game/Jamar_B/Effects/Niagra/NS_FX.NS_FX" (Transformation|GetActorLocation) "0, 0, 0" "0.500000,0.500000,0.500000")
    (Actor|DestroyActor)))

(fn ConstructionScript)