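; Collectible ship part that the player picks up by touching it.
; On BeginPlay it caches the first BP_HUDmanager actor found in the level.
; When the player character overlaps its Box, it calls AddGear on that manager, destroys itself and prints a pickup message.
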(event OnComponentBeginOverlap(Box)
  (params (OverlappedComponent :type Primitive%20Component%20Object%20Reference) (OtherActor :type Actor%20Object%20Reference) (OtherComp :type Primitive%20Component%20Object%20Reference) (OtherBodyIndex :type Integer) (bFromSweep :type Boolean) (SweepResult :type Hit%20Result%20Structure%20%28by%20ref%29))
  (if (== OtherActor (Game|GetPlayerCharacter 0))
    (Default|AddGear (Variables|Default|GetMyHUDManager))
    (Actor|DestroyActor)
    (Development|PrintString "You collected a ship part!")))

(event EventBeginPlay
  (bind _outactors (Actor|GetAllActorsOfClass "/Game/Userinterface_bars/BP_HUDmanager.BP_HUDmanager_C"))
  (Variables|Default|SetMyHUDManager (Utilities|Array|Get(acopy) _outactors)))

(fn ConstructionScript)