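; Overview showcase lighting actor that lays out a grid of spotlights over all BP_Category_Platform actors in the level.
; Its construction script rebuilds the spotlight components from the platforms' combined bounds, deriving grid density from a gap threshold and placing them at a set height.
; Shared variables drive each light's rotation, intensity, cone, source and color.
; BakeLights replaces the generated components with standalone BP_Spotlight actors, then destroys this actor.
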(event EventBeginPlay)

(event Collision|EventActorBeginOverlap
  (params (OtherActor :type Actor%20Object%20Reference)))

(event EventTick
  (params (DeltaSeconds :type Float%20%28single-precision%29)))

(fn ConstructionScript
  (Rendering|Components|Sprite|SetSprite (Variables|Default|GetBillboard) "/Game/TextureSets_MGN/Library_MGN/Showcase/Overview/Texture/T_LightSystem.T_LightSystem")
  (CallFunction|SetupOverviewLights))

(fn SetupOverviewLights
  (bind _allspotlights (Variables|Default|GetAllSpotLights))
  (Utilities|Array|Clear (Variables|Default|GetAllPlatforms))
  (for _array_element _allspotlights
    (Utilities|IsValid _array_element
      (:Is%20Valid
        (Components|DestroyComponent _array_element))))
  (Utilities|FlowControl|Sequence
    (:then_0
      (Utilities|Array|Clear _allspotlights))
    (:then_1
      (bind _outactors (Actor|GetAllActorsOfClass self "/Game/TextureSets_MGN/Library_MGN/Showcase/Overview/Blueprint/BP_Category_Platform.BP_Category_Platform_C"))
      (bind _output_get (Variables|Default|SetAllPlatforms _outactors))
      (for _array_element_2 _output_get
        (Utilities|Array|Add (LocalVariables|GetLocal_allActors) _array_element_2))
      (Utilities|FlowControl|Sequence
        (:then_0
          ;[0.07812 0.07812 0.07812] Find bound of all showcase assets on the platform
          (bind (_center _boxextent) (Collision|GetActorArrayBounds (LocalVariables|GetLocal_allActors)))
          (LocalVariables|SetLocal_platformsCenter _center)
          (LocalVariables|SetLocal_platformsExtent _boxextent)
          (LocalVariables|SetLocal_platformsClosestLeftTop (+ (LocalVariables|GetLocal_platformsCenter) (Math|Vector|MakeVector (* (.x (LocalVariables|GetLocal_platformsExtent)) -1.0) (.y (LocalVariables|GetLocal_platformsExtent)) (.z (LocalVariables|GetLocal_platformsExtent)))))
          (LocalVariables|SetLocal_platformsClosestRightTop (+ (LocalVariables|GetLocal_platformsCenter) (Math|Vector|MakeVector (.x (LocalVariables|GetLocal_platformsExtent)) (.y (LocalVariables|GetLocal_platformsExtent)) (.z (LocalVariables|GetLocal_platformsExtent)))))
          (LocalVariables|SetLocal_platformsFurthestLeftTop (+ (LocalVariables|GetLocal_platformsCenter) (Math|Vector|MakeVector (* (.x (LocalVariables|GetLocal_platformsExtent)) -1.0) (* (.y (LocalVariables|GetLocal_platformsExtent)) -1.0) (.z (LocalVariables|GetLocal_platformsExtent)))))
          (LocalVariables|SetLocal_platformsFurthestRightTop (+ (LocalVariables|GetLocal_platformsCenter) (Math|Vector|MakeVector (* (.x (LocalVariables|GetLocal_platformsExtent)) 1.0) (* (.y (LocalVariables|GetLocal_platformsExtent)) -1.0) (.z (LocalVariables|GetLocal_platformsExtent))))))
        (:then_1
          ;[0.07292 0.07292 0.07292] Light Count
          (LocalVariables|SetLocal_widthCount (Math|Float|Truncate (/ (Math|Vector|VectorLength (- (LocalVariables|GetLocal_platformsClosestLeftTop) (LocalVariables|GetLocal_platformsClosestRightTop))) (Variables|Lights|GetSpotLightGapThreshold))))
          (LocalVariables|SetLocal_depthCount (Math|Float|Truncate (/ (Math|Vector|VectorLength (- (LocalVariables|GetLocal_platformsFurthestRightTop) (LocalVariables|GetLocal_platformsClosestRightTop))) (Variables|Lights|GetSpotLightGapThreshold)))))
        (:then_2
          (Utilities|FlowControl|Sequence
            (:then_0
              (for _index (range 0 (+ (LocalVariables|GetLocal_widthCount) 1))
                (Utilities|Array|Add (LocalVariables|GetLocal_lightList) (Math|Vector|MakeVector (.X (Math|Vector|BreakVector (+ (LocalVariables|GetLocal_platformsClosestLeftTop) (* (Math|Vector|Normalize (- (LocalVariables|GetLocal_platformsClosestRightTop) (LocalVariables|GetLocal_platformsClosestLeftTop))) (/ (Math|Vector|VectorLength (- (LocalVariables|GetLocal_platformsClosestRightTop) (LocalVariables|GetLocal_platformsClosestLeftTop))) (+ (LocalVariables|GetLocal_widthCount) 1)) _index)))) (.Y (Math|Vector|BreakVector (+ (LocalVariables|GetLocal_platformsClosestLeftTop) (* (Math|Vector|Normalize (- (LocalVariables|GetLocal_platformsClosestRightTop) (LocalVariables|GetLocal_platformsClosestLeftTop))) (/ (Math|Vector|VectorLength (- (LocalVariables|GetLocal_platformsClosestRightTop) (LocalVariables|GetLocal_platformsClosestLeftTop))) (+ (LocalVariables|GetLocal_widthCount) 1)) _index)))) (Variables|Lights|GetHeight)))
                (for _index_2 (range 0 (+ (LocalVariables|GetLocal_depthCount) 1))
                  (Utilities|Array|Add (LocalVariables|GetLocal_lightList) (Math|Vector|MakeVector (.x (+ (+ (LocalVariables|GetLocal_platformsClosestLeftTop) (* (Math|Vector|Normalize (- (LocalVariables|GetLocal_platformsClosestRightTop) (LocalVariables|GetLocal_platformsClosestLeftTop))) (/ (Math|Vector|VectorLength (- (LocalVariables|GetLocal_platformsClosestRightTop) (LocalVariables|GetLocal_platformsClosestLeftTop))) (+ (LocalVariables|GetLocal_widthCount) 1)) _index)) (* (Math|Vector|Normalize (- (LocalVariables|GetLocal_platformsFurthestRightTop) (LocalVariables|GetLocal_platformsClosestRightTop))) (/ (Math|Vector|VectorLength (- (LocalVariables|GetLocal_platformsClosestRightTop) (LocalVariables|GetLocal_platformsFurthestRightTop))) (+ (LocalVariables|GetLocal_depthCount) 1)) _index_2))) (.y (+ (+ (LocalVariables|GetLocal_platformsClosestLeftTop) (* (Math|Vector|Normalize (- (LocalVariables|GetLocal_platformsClosestRightTop) (LocalVariables|GetLocal_platformsClosestLeftTop))) (/ (Math|Vector|VectorLength (- (LocalVariables|GetLocal_platformsClosestRightTop) (LocalVariables|GetLocal_platformsClosestLeftTop))) (+ (LocalVariables|GetLocal_widthCount) 1)) _index)) (* (Math|Vector|Normalize (- (LocalVariables|GetLocal_platformsFurthestRightTop) (LocalVariables|GetLocal_platformsClosestRightTop))) (/ (Math|Vector|VectorLength (- (LocalVariables|GetLocal_platformsClosestRightTop) (LocalVariables|GetLocal_platformsFurthestRightTop))) (+ (LocalVariables|GetLocal_depthCount) 1)) _index_2))) (Variables|Lights|GetHeight))))))
            (:then_2
              (for _array_element_3 (LocalVariables|GetLocal_lightList)
                (bind _returnvalue (AddComponent|AddSpotLightComponent false))
                (bind _output_get_2 (LocalVariables|SetLocal_currentSpotLight _returnvalue))
                (Utilities|Array|Add (Variables|Default|GetAllSpotLights) _output_get_2)
                (Transformation|SetWorldTransform (LocalVariables|GetLocal_currentSpotLight) (Math|Transform|MakeTransform _array_element_3 (Variables|Lights|GetRotation)) false false)
                (CallFunction|SetLightVariables (LocalVariables|GetLocal_currentSpotLight))))))))))

(fn SetLightVariables
  (params (Target :type Spot%20Light%20Component%20Object%20Reference%20%28by%20ref%29))
  (Rendering|Components|Light|SetIntensity Target (Variables|Lights|GetIntensity))
  (Class|LocalLightComponent|SetIntensityUnits Target "Candelas")
  (Rendering|Lighting|SetAttenuationRadius Target (Variables|Lights|GetAttenuationRadius))
  (Rendering|Lighting|SetInnerConeAngle Target (Variables|Lights|GetInnerConeAngle))
  (Rendering|Lighting|SetOuterConeAngle Target (Variables|Lights|GetOuterConeAngle))
  (Class|PointLightComponent|SetSoftSourceRadius Target (Variables|Lights|GetSoftSourceRadius))
  (Class|PointLightComponent|SetSourceLength Target (Variables|Lights|GetSource%20Length))
  (Rendering|Components|Light|SetLightColor Target (Variables|Lights|GetColor) true))

(fn BakeLights[WillDestroyThisBP]
  (CallFunction|SetupOverviewLights)
  (for _array_element (Variables|Default|GetAllSpotLights)
    (bind _returnvalue (Game|SpawnActorfromClass "/Game/TextureSets_MGN/Library_MGN/Showcase/Overview/Blueprint/BP_Spotlight.BP_Spotlight_C" (Transformation|GetWorldTransform _array_element) "Undefined" "MultiplyWithRoot" 0 0))
    (Transformation|SetActorTransform _returnvalue (Transformation|GetWorldTransform _array_element))
    (bind _output_get (LocalVariables|SetLocal_spotLight (Variables|/Script/Engine.SpotLight|GetSpotLightComponent _returnvalue)))
    (CallFunction|SetLightVariables _output_get))
  (Actor|DestroyActor))