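; BP_PuzzleTrigger is a trigger volume that presents a puzzle to the player character Bp_Lyla and opens a linked Door once it is solved.
; Overlapping its Box while unsolved creates the WBP_Puzzle widget, switches to UI-only input with a mouse cursor, and disables and halts Lyla.
; The widget's OnPuzzleSolved dispatcher marks the trigger solved and opens the Door; this file does not restore input.
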(event OnComponentBeginOverlap(Box)
  (params (OverlappedComponent :type Primitive%20Component%20Object%20Reference) (OtherActor :type Actor%20Object%20Reference) (OtherComp :type Primitive%20Component%20Object%20Reference) (OtherBodyIndex :type Integer) (bFromSweep :type Boolean) (SweepResult :type Hit%20Result%20Structure%20%28by%20ref%29))
  (bind _returnvalue (Game|GetPlayerController 0))
  (bind _asbp_lyla (Utilities|Casting|CastToBp_Lyla OtherActor))
  (if (not (Variables|Default|GetbSolved))
    (bind _returnvalue_2 (UserInterface|CreateWidget "/Game/Puzzles/WBP_Puzzle.WBP_Puzzle_C" _returnvalue))
    (EventDispatchers|AssignOnPuzzleSolved _returnvalue_2 (delegate Custom|OnPuzzleSolved_Event))
    (UserInterface|Viewport|AddtoViewport _returnvalue_2 0)
    (Input|SetInputModeUIOnly _returnvalue _returnvalue_2 "DoNotLock" false)
    (Variables|/Script/Engine.PlayerController|SetbShowMouseCursor _returnvalue true)
    (Input|DisableInput _asbp_lyla _returnvalue)
    (Components|Movement|StopMovementImmediately (Variables|/Script/Engine.Character|GetCharacterMovement _asbp_lyla))))

(event Custom|OnPuzzleSolved_Event
  (Variables|Default|SetbSolved true)
  (Default|OpenDoor (Variables|Default|GetDoor)))

(event EventBeginPlay)

(event Collision|EventActorBeginOverlap
  (params (OtherActor :type Actor%20Object%20Reference)))

(event EventTick
  (params (DeltaSeconds :type Float%20%28single-precision%29)))

(fn ConstructionScript)