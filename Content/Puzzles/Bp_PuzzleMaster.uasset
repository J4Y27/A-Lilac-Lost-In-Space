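; Puzzle manager Blueprint that checks whether the pipes in a pipe puzzle are set correctly.
; PipePuzzleCheck asks each entry in Pipes to validate itself and increments NumOfCorrectPipes for each pass, without resetting the count first.
; When the count equals the number of pipes it only sets the counter to a fixed value, with no other solved response.
; ValidatePipePuzzle is a stub that always returns false.
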(event EventPipePuzzleCheck
  (bind _pipes (Variables|Default|GetPipes))
  (for _array_element _pipes
    (bind _correct_ (Class|IntInteract|ValidatePipePuzzle(Message) _array_element))
    (if _correct_
      (Math|Integer|IncrementInt (Variables|Default|GetNum%20Of%20Correct%20Pipes))))
  (if (== (Utilities|Array|Length _pipes) (Variables|Default|GetNum%20Of%20Correct%20Pipes))
    (Variables|Default|SetNum%20Of%20Correct%20Pipes 3)))

(fn ConstructionScript)

(fn ValidatePipePuzzle
  (return false))