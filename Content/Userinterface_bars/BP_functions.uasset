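; Blueprint helper functions for reaching and toggling the player's HUD.
; GetMyHUD casts player controller 0's HUD to BP_UIManager and returns it.
; HideMyHUD and ShowMyHUD use that getter to set the manager's HUDWidgetRef to Hidden or Visible.
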(fn GetMyHUD
  (bind _asbp_uimanager (Utilities|Casting|CastToBP_UIManager (HUD|GetHUD (Game|GetPlayerController 0))))
  (return _asbp_uimanager))

(fn HideMyHUD
  (Widget|SetVisibility (Variables|/Game/Userinterface_bars/BP_UIManager.BP_UIManager_C|GetHUD_WidgetRef (CallFunction|GetMyHUD)) "Hidden")
  (return))

(fn ShowMyHUD
  (Widget|SetVisibility (Variables|/Game/Userinterface_bars/BP_UIManager.BP_UIManager_C|GetHUD_WidgetRef (CallFunction|GetMyHUD)) "Visible")
  (return))